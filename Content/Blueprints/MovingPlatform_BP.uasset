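; Moving platform actor that shuttles its Platform component back and forth between a start and an end location.
; BeginPlay stores the component's world location as the start, then binds and immediately calls the Move dispatcher.
; The bound event loops forever through eased, timed MoveComponentTo moves with a short pause at each end.
; Both targets are applied as relative locations, although the start is captured in world space.
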(event `self.ReceiveBeginPlay`
  (set `self.StartLocation` (`SceneComponent.K2_GetComponentLocation` (`self.Platform`)))
  (add `self.Move` (delegate `Move_Event`))
  (`self.Move`))

(event `Move_Event`
  (`KismetSystemLibrary.MoveComponentTo` (`self.Platform`) (`self.EndLocation`) (struct) true true 2.0 :!label _label)
  (`KismetSystemLibrary.Delay` 0.2)
  (`KismetSystemLibrary.MoveComponentTo` (`self.Platform`) (`self.StartLocation`) (struct) true true 2.0)
  (`KismetSystemLibrary.Delay` 0.2)
  (goto _label))

(fn `UserConstructionScript`)