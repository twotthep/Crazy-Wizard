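; Boss Blueprint that takes damage from physics balls and displays its health on a widget bar.
; When a PhysicsBallBP enters the box it loses PlayerDMG health and sets a ShowHP flag, cleared on exit, with debug prints for both.
; Every Tick recomputes the health fraction and pushes it to the BossUI progress bar in the HPBar component.
; ShowHP is not read here, and no death handling is present.
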(event `self.ReceiveBeginPlay`)

(event `self.Box.OnComponentBeginOverlap`
  (params (OverlappedComponent :type "PrimitiveComponent Object Reference") (OtherActor :type "Actor Object Reference") (OtherComp :type "PrimitiveComponent Object Reference") (OtherBodyIndex :type Integer) (bFromSweep :type Boolean) (SweepResult :type "HitResult Structure (by ref)"))
  (cast `/Game/RollingBP/Blueprints/PhysicsBallBP` OtherActor)
  (set `self.showHP` true)
  (`KismetSystemLibrary.PrintString` "Show HP")
  (set `self.currentHealth` (- (`self.currentHealth`) (`self.playerDMG`))))

(event `self.Box.OnComponentEndOverlap`
  (params (OverlappedComponent :type "PrimitiveComponent Object Reference") (OtherActor :type "Actor Object Reference") (OtherComp :type "PrimitiveComponent Object Reference") (OtherBodyIndex :type Integer))
  (cast `/Game/RollingBP/Blueprints/PhysicsBallBP` OtherActor)
  (set `self.showHP` false)
  (`KismetSystemLibrary.PrintString` "Hide HP"))

(event `self.ReceiveTick`
  (params (DeltaSeconds :type "Float (single-precision)"))
  (`self.healthToPercent`)
  (bind _asboss_ui (cast `/Game/Blueprints/Character/Boss/BossUI` (`WidgetComponent.GetUserWidgetObject` (`self.HPBar`))))
  (`ProgressBar.SetPercent` (`/Game/Blueprints/Character/Boss/BossUI.ProgressBar_167` _asboss_ui) (`self.healthPercentage`)))

(fn `healthToPercent`
  (set `self.healthPercentage` (/ (`self.currentHealth`) (`self.maxHealth`))))

(fn `UserConstructionScript`)